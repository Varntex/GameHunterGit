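; BP_TreeBlob is a shootable tree that switches to a burned look once its health is depleted.
; BeginPlay randomly picks one of two tree variants and hides the other, along with both burned versions.
; GetShot subtracts incoming damage from Health and returns true.
; Tick polls Health and, once it drops below zero, uses a DoOnce to swap the chosen tree for its matching burned version.
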(event `self.ReceiveBeginPlay`
  (bind _tree1 (`self.Tree1`))
  (bind _tree2 (`self.Tree2`))
  (`SceneComponent.SetVisibility` (`self.TreeBurned1`) false false)
  (`SceneComponent.SetVisibility` (`self.TreeBurned2`) false false)
  (bind _output_get (set `self.Variant` (`KismetMathLibrary.RandomIntegerInRange` 0 1)))
  (if (== _output_get 0)
    (set `self.TreeVariant` _tree1)
    (`SceneComponent.SetVisibility` _tree2 false false)
    (elif (== _output_get 1)
      (set `self.TreeVariant` _tree2)
      (`SceneComponent.SetVisibility` _tree1 false false))))

(event `self.ReceiveTick`
  (params (DeltaSeconds :type "Float (single-precision)"))
  (bind _variant (`self.Variant`))
  (if (not (>= (`self.Health`) 0))
    (`/Engine/EditorBlueprintResources/StandardMacros.DoOnce` false
      (:`Completed`
        (`SceneComponent.SetVisibility` (`self.TreeVariant`) false false)
        (if (== _variant 0)
          (`SceneComponent.SetVisibility` (`self.TreeBurned1`) true false)
          (elif (== _variant 1)
            (`SceneComponent.SetVisibility` (`self.TreeBurned2`) true false)))))))

(fn `GetShot`
  (params (Damage :type Integer))
  (returns (`GotShot?` :type Boolean))
  (set `self.Health` (- (`self.Health`) Damage))
  (return true))

(fn `UserConstructionScript`)