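; Campfire actor that repeatedly damages an overlapping actor implementing Interface_TakeDamage.
; Begin and end overlap events toggle a damage flag for such actors, while every begin overlap overwrites the single stored target.
; While the flag is set, Tick sends TakeDamageMessage to that target, throttled by a DoOnce that resets after a short Delay.
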(event `self.ReceiveActorBeginOverlap`
  (params (OtherActor :type "Actor Object Reference"))
  (set `self.Other Actor` OtherActor)
  (if (`KismetSystemLibrary.DoesImplementInterface` OtherActor "/Game/ThirdPersonBP/Blueprints/Interface_TakeDamage.Interface_TakeDamage_C")
    (set `self.DealingDamage` true)))

(event `self.ReceiveActorEndOverlap`
  (params (OtherActor :type "Actor Object Reference"))
  (if (`KismetSystemLibrary.DoesImplementInterface` OtherActor "/Game/ThirdPersonBP/Blueprints/Interface_TakeDamage.Interface_TakeDamage_C")
    (set `self.DealingDamage` false)))

(event `self.ReceiveTick`
  (params (DeltaSeconds :type "Float (single-precision)"))
  (if (`self.DealingDamage`)
    (`/Engine/EditorBlueprintResources/StandardMacros.DoOnce` false :!label _label
      (:`Completed`
        (message `/Game/ThirdPersonBP/Blueprints/Interface_TakeDamage.TakeDamage` (`self.Other Actor`) 1)
        (`KismetSystemLibrary.Delay` 0.1)
        (goto _label :!via `Reset`)))))

(fn `UserConstructionScript`)