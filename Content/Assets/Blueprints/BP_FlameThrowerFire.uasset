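; BP_FlameThrowerFire is a short-lived actor, by its name a flamethrower fire puff, that grows over its lifetime and then removes itself.
; BeginPlay destroys the actor after a one-second delay.
; Tick uses a DoOnce reset by a short delay to throttle growth, adding GrowthFloat to each axis of the root component's world scale in timed steps rather than every frame.
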(event `self.ReceiveBeginPlay`
  (`KismetSystemLibrary.Delay` 1.0)
  (`self.K2_DestroyActor`))

(event `self.ReceiveTick`
  (params (DeltaSeconds :type "Float (single-precision)"))
  (bind _defaultsceneroot (`self.DefaultSceneRoot`))
  (bind _growthfloat (`self.GrowthFloat`))
  (`/Engine/EditorBlueprintResources/StandardMacros.DoOnce` false :!label _label
    (:`Completed`
      (`SceneComponent.SetWorldScale3D` _defaultsceneroot (`KismetMathLibrary.MakeVector` (+ (.x (`SceneComponent.K2_GetComponentScale` _defaultsceneroot)) _growthfloat) (+ (.y (`SceneComponent.K2_GetComponentScale` _defaultsceneroot)) _growthfloat) (+ (.z (`SceneComponent.K2_GetComponentScale` _defaultsceneroot)) _growthfloat)))
      (`KismetSystemLibrary.Delay` 0.1)
      (goto _label :!via `Reset`))))

(fn `UserConstructionScript`)