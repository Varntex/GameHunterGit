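; BP_Tree is a tree that takes damage from shots and topples when its health runs out.
; GetShot subtracts the damage from Health and always returns false.
; Tick polls Health and, once it drops below zero, a DoOnce snaps the root to a fallen pitch with a random yaw, without animation or physics.
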(event `self.ReceiveTick`
  (params (DeltaSeconds :type "Float (single-precision)"))
  (if (not (>= (`self.Health`) 0))
    (`/Engine/EditorBlueprintResources/StandardMacros.DoOnce` false
      (:`Completed`
        (`SceneComponent.K2_SetWorldRotation` (`self.DefaultSceneRoot`) (`KismetMathLibrary.MakeRotator` 0.0 100.0 (`KismetMathLibrary.RandomFloatInRange` 0.0 360.0)) false false)))))

(fn `GetShot`
  (params (Damage :type Integer))
  (returns (`GotShot?` :type Boolean))
  (set `self.Health` (- (`self.Health`) Damage))
  (return false))

(fn `UserConstructionScript`)