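; BP_WaterTrigger is a trigger actor for water that damages the player character on entry and reports when the player is in it.
; Beginning an overlap sends BP_PlayerCharacter a large damage message and sets its water state on, while ending the overlap sets that state off.
; BeginPlay caches the player and the first child component of its mesh, though the overlap logic uses neither reference.
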(event `self.ReceiveBeginPlay`
  (bind _asbp_player_character (cast `/Game/ThirdPersonBP/Blueprints/BP_PlayerCharacter` (`GameplayStatics.GetPlayerCharacter` 0)))
  (set `self.As BP_PlayerCharacter` _asbp_player_character)
  (set `self.PlayerMesh` (`SceneComponent.GetChildComponent` (`Character.Mesh` _asbp_player_character) 0)))

(event `self.ReceiveActorBeginOverlap`
  (params (OtherActor :type "Actor Object Reference"))
  (bind _asbp_player_character (cast `/Game/ThirdPersonBP/Blueprints/BP_PlayerCharacter` OtherActor))
  (message `/Game/ThirdPersonBP/Blueprints/Interface_TakeDamage.TakeDamage` _asbp_player_character 100)
  (message `/Game/ThirdPersonBP/Blueprints/Interface_Water.Water` _asbp_player_character true))

(event `self.ReceiveActorEndOverlap`
  (params (OtherActor :type "Actor Object Reference"))
  (bind _asbp_player_character (cast `/Game/ThirdPersonBP/Blueprints/BP_PlayerCharacter` OtherActor))
  (message `/Game/ThirdPersonBP/Blueprints/Interface_Water.Water` _asbp_player_character false))

(fn `UserConstructionScript`)