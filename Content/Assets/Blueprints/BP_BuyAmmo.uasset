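; BP_BuyAmmo is an ammo purchase whose Use function reports a coin cost and the type of purchase.
; Use casts the player character to BP_PlayerCharacter and checks for an equipped rifle, machine gun, rocket launcher or flamethrower.
; Any of these yields a fixed coin deduction, otherwise zero.
; BoughtAmmo returns true in both cases, leaving coin and ammo changes outside this Blueprint.
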(fn `Use`
  (returns (CoinsAmount :type Integer) (`BoughtAmmo?` :type Boolean) (`BoughtWeapon?` :type Boolean) (`BoughtGrenades?` :type Boolean) (`FoundFlamethrower?` :type Boolean))
  (bind _asbp_player_character (cast `/Game/ThirdPersonBP/Blueprints/BP_PlayerCharacter` (`GameplayStatics.GetPlayerCharacter` 0)))
  (if (`/Game/ThirdPersonBP/Blueprints/BP_PlayerCharacter.RifleEquipped` _asbp_player_character)
    (set `self.Coins Amount` -75 :!label _label)
    (elif (`/Game/ThirdPersonBP/Blueprints/BP_PlayerCharacter.MachineGunEquipped` _asbp_player_character)
      (goto _label)
      (elif (`/Game/ThirdPersonBP/Blueprints/BP_PlayerCharacter.RocketLauncherEquipped` _asbp_player_character)
        (goto _label)
        (elif (`/Game/ThirdPersonBP/Blueprints/BP_PlayerCharacter.FlamethrowerEquipped` _asbp_player_character)
          (goto _label)
          (else
            (set `self.Coins Amount` 0))))))
  (return (`self.Coins Amount`) true false false false))

(fn `UserConstructionScript`)