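; BP_CampWeapons is a camp weapon display that shows the rifle and flamethrower the player does not have equipped.
; Every Tick it casts the player character to BP_PlayerCharacter and reads its equip and unlock flags to set component visibility.
; The Rifle shows whenever it is unequipped, while the Flamethrower also requires being unlocked.
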(event `self.ReceiveTick`
  (params (DeltaSeconds :type "Float (single-precision)"))
  (bind _rifle (`self.Rifle`))
  (bind _flamethrower (`self.Flamethrower`))
  (bind _asbp_player_character (cast `/Game/ThirdPersonBP/Blueprints/BP_PlayerCharacter` (`GameplayStatics.GetPlayerCharacter` 0)))
  (`|ExecutionSequence`
    (:`then_0`
      (if (`/Game/ThirdPersonBP/Blueprints/BP_PlayerCharacter.RifleEquipped` _asbp_player_character)
        (`SceneComponent.SetVisibility` _rifle false false)
        (else
          (`SceneComponent.SetVisibility` _rifle true false))))
    (:`then_1`
      (if (`/Game/ThirdPersonBP/Blueprints/BP_PlayerCharacter.FlamethrowerEquipped` _asbp_player_character)
        (`SceneComponent.SetVisibility` _flamethrower false false :!label _label)
        (elif (`/Game/ThirdPersonBP/Blueprints/BP_PlayerCharacter.FlamethrowerUnlocked` _asbp_player_character)
          (`SceneComponent.SetVisibility` _flamethrower true false)
          (else
            (goto _label)))))))

(fn `UserConstructionScript`)