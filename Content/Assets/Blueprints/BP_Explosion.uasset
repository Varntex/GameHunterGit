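; BP_Explosion is a short-lived explosion actor that damages and pushes whatever overlaps it, then destroys itself when its particle system finishes.
; Damage is gated by CanDamage, which switches off shortly after BeginPlay.
; Each qualifying overlap sends GetShot and TakeDamage interface messages to the other actor.
; It also impulses all overlapping physics-simulating components away from the center, with force growing with distance rather than falling off.
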(event `self.ParticleSystem.OnSystemFinished`
  (params (PSystem :type "ParticleSystemComponent Object Reference"))
  (`self.K2_DestroyActor`))

(event `self.ReceiveBeginPlay`
  (`KismetSystemLibrary.Delay` 0.5)
  (set `self.CanDamage` false))

(event `self.ReceiveActorBeginOverlap`
  (params (OtherActor :type "Actor Object Reference"))
  (if (`self.CanDamage`)
    (`|ExecutionSequence`
      (:`then_0`
        (if (`KismetSystemLibrary.DoesImplementInterface` OtherActor "/Game/Assets/Animals/Interface_GetShot.Interface_GetShot_C")
          (message `/Game/Assets/Animals/Interface_GetShot.GetShot` OtherActor 100)))
      (:`then_1`
        (if (`KismetSystemLibrary.DoesImplementInterface` OtherActor "/Game/ThirdPersonBP/Blueprints/Interface_TakeDamage.Interface_TakeDamage_C")
          (message `/Game/ThirdPersonBP/Blueprints/Interface_TakeDamage.TakeDamage` OtherActor 100)))
      (:`then_2`
        (for _array_element (`self.GetOverlappingComponents`)
          (if (`SceneComponent.IsSimulatingPhysics` _array_element "None")
            (`PrimitiveComponent.AddImpulse` _array_element (* (- (`self.K2_GetActorLocation`) (`SceneComponent.K2_GetComponentLocation` _array_element)) -100.0) "None" false)))))))

(fn `UserConstructionScript`)