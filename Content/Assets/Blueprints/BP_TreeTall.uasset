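; BP_TreeTall is a destructible tall tree that swaps to a burned mesh when its health runs out.
; BeginPlay randomly keeps one of four tree meshes, hiding and disabling collision on the others, and hides both burned meshes.
; GetShot subtracts damage from Health and returns true.
; Tick polls Health and, once below zero, hides the live tree and shows one of two burned meshes, each shared by two variants.
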(event `self.ReceiveBeginPlay`
  (bind _tree1 (`self.Tree1`))
  (bind _tree2 (`self.Tree2`))
  (bind _tree3 (`self.Tree3`))
  (bind _tree4 (`self.Tree4`))
  (`SceneComponent.SetVisibility` (`self.TreeBurned1`) false false)
  (`SceneComponent.SetVisibility` (`self.TreeBurned2`) false false)
  (bind _output_get (set `self.Variant` (`KismetMathLibrary.RandomIntegerInRange` 0 3)))
  (if (== _output_get 0)
    (set `self.TreeVariant` _tree1)
    (`SceneComponent.SetVisibility` _tree2 false false)
    (`SceneComponent.SetVisibility` _tree3 false false)
    (`SceneComponent.SetVisibility` _tree4 false false)
    (`PrimitiveComponent.SetCollisionEnabled` _tree2 "NoCollision")
    (`PrimitiveComponent.SetCollisionEnabled` _tree3 "NoCollision")
    (`PrimitiveComponent.SetCollisionEnabled` _tree4 "NoCollision")
    (elif (== _output_get 1)
      (set `self.TreeVariant` _tree2)
      (`SceneComponent.SetVisibility` _tree1 false false)
      (`SceneComponent.SetVisibility` _tree3 false false)
      (`SceneComponent.SetVisibility` _tree4 false false)
      (`PrimitiveComponent.SetCollisionEnabled` _tree1 "NoCollision")
      (`PrimitiveComponent.SetCollisionEnabled` _tree3 "NoCollision")
      (`PrimitiveComponent.SetCollisionEnabled` _tree4 "NoCollision")
      (elif (== _output_get 2)
        (set `self.TreeVariant` _tree3)
        (`SceneComponent.SetVisibility` _tree1 false false)
        (`SceneComponent.SetVisibility` _tree2 false false)
        (`SceneComponent.SetVisibility` _tree4 false false)
        (`PrimitiveComponent.SetCollisionEnabled` _tree1 "NoCollision")
        (`PrimitiveComponent.SetCollisionEnabled` _tree2 "NoCollision")
        (`PrimitiveComponent.SetCollisionEnabled` _tree4 "NoCollision")
        (elif (== _output_get 3)
          (set `self.TreeVariant` _tree4)
          (`SceneComponent.SetVisibility` _tree1 false false)
          (`SceneComponent.SetVisibility` _tree2 false false)
          (`SceneComponent.SetVisibility` _tree3 false false)
          (`PrimitiveComponent.SetCollisionEnabled` _tree1 "NoCollision")
          (`PrimitiveComponent.SetCollisionEnabled` _tree2 "NoCollision")
          (`PrimitiveComponent.SetCollisionEnabled` _tree3 "NoCollision"))))))

(event `self.ReceiveTick`
  (params (DeltaSeconds :type "Float (single-precision)"))
  (bind _treevariant (`self.TreeVariant`))
  (bind _variant (`self.Variant`))
  (if (not (>= (`self.Health`) 0))
    (`/Engine/EditorBlueprintResources/StandardMacros.DoOnce` false
      (:`Completed`
        (`SceneComponent.SetVisibility` _treevariant false false)
        (`PrimitiveComponent.SetCollisionEnabled` _treevariant "NoCollision")
        (if (== _variant 0)
          (`SceneComponent.SetVisibility` (`self.TreeBurned1`) true false :!label _label)
          (elif (== _variant 1)
            (goto _label)
            (elif (== _variant 2)
              (`SceneComponent.SetVisibility` (`self.TreeBurned2`) true false :!label _label_2)
              (elif (== _variant 3)
                (goto _label_2)))))))))

(fn `GetShot`
  (params (Damage :type Integer))
  (returns (`GotShot?` :type Boolean))
  (set `self.Health` (- (`self.Health`) Damage))
  (return true))

(fn `UserConstructionScript`)