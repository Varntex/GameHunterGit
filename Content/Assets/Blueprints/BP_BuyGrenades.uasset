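; BP_BuyGrenades is a purchase point where the player buys grenades.
; Its Use function only returns an Amount of -15 with the BoughtGrenades flag set, leaving the transaction to the caller.
; Every tick it turns its text toward the player's camera and swaps three pairs of grenade meshes between grenade and "don't have" materials at rising GrenadeAmmo thresholds, showing the player's current stock.
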(event `self.ReceiveTick`
  (params (DeltaSeconds :type "Float (single-precision)"))
  (bind _grenade3 (`self.Grenade3`))
  (bind _grenade4 (`self.Grenade4`))
  (bind _grenade (`self.Grenade`))
  (bind _asbp_player_character (cast `/Game/ThirdPersonBP/Blueprints/BP_PlayerCharacter` (`GameplayStatics.GetPlayerCharacter` 0)))
  (`SceneComponent.K2_SetWorldRotation` (`self.Text`) (`KismetMathLibrary.FindLookAtRotation` (`self.K2_GetActorLocation`) (`SceneComponent.K2_GetComponentLocation` (`/Game/ThirdPersonBP/Blueprints/Ue4ASP_Character.PlayerCamera` _asbp_player_character))) false false)
  (`|ExecutionSequence`
    (:`then_0`
      (bind _grenadeammo (`/Game/ThirdPersonBP/Blueprints/BP_PlayerCharacter.GrenadeAmmo` _asbp_player_character))
      (if (> _grenadeammo 0)
        (`PrimitiveComponent.SetMaterial` _grenade 0 "/Game/Assets/Character/Weapons/Grenade/MM_prop_grenade_02.MM_prop_grenade_02")
        (`PrimitiveComponent.SetMaterial` (`self.Grenade2`) 0 "/Game/Assets/Character/Weapons/Grenade/MM_prop_grenade_02.MM_prop_grenade_02")
        (else
          (`PrimitiveComponent.SetMaterial` _grenade 0 "/Game/Assets/Paceholders/Camp/MA_DontHave.MA_DontHave")
          (`PrimitiveComponent.SetMaterial` (`self.Grenade2`) 0 "/Game/Assets/Paceholders/Camp/MA_DontHave.MA_DontHave"))))
    (:`then_1`
      (if (> _grenadeammo 2)
        (`PrimitiveComponent.SetMaterial` _grenade3 0 "/Game/Assets/Character/Weapons/Grenade/MM_prop_grenade_02.MM_prop_grenade_02")
        (`PrimitiveComponent.SetMaterial` (`self.Grenade1`) 0 "/Game/Assets/Character/Weapons/Grenade/MM_prop_grenade_02.MM_prop_grenade_02")
        (else
          (`PrimitiveComponent.SetMaterial` _grenade3 0 "/Game/Assets/Paceholders/Camp/MA_DontHave.MA_DontHave")
          (`PrimitiveComponent.SetMaterial` (`self.Grenade1`) 0 "/Game/Assets/Paceholders/Camp/MA_DontHave.MA_DontHave"))))
    (:`then_2`
      (if (> _grenadeammo 4)
        (`PrimitiveComponent.SetMaterial` _grenade4 0 "/Game/Assets/Character/Weapons/Grenade/MM_prop_grenade_02.MM_prop_grenade_02")
        (`PrimitiveComponent.SetMaterial` (`self.Grenade5`) 0 "/Game/Assets/Character/Weapons/Grenade/MM_prop_grenade_02.MM_prop_grenade_02")
        (else
          (`PrimitiveComponent.SetMaterial` _grenade4 0 "/Game/Assets/Paceholders/Camp/MA_DontHave.MA_DontHave")
          (`PrimitiveComponent.SetMaterial` (`self.Grenade5`) 0 "/Game/Assets/Paceholders/Camp/MA_DontHave.MA_DontHave"))))))

(fn `Use`
  (returns (Amount :type Integer) (`SoldMeat?` :type Boolean) (`BoughtAmmo?` :type Boolean) (`BoughtWeapon?` :type Boolean) (`BoughtGrenades?` :type Boolean) (`FoundFlamethrower?` :type Boolean) (`PickedUpMeat?` :type Boolean))
  (return -15 false false false true false false))

(fn `UserConstructionScript`)