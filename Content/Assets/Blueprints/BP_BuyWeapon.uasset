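; BP_BuyWeapon is a shop interactable that sells weapon upgrades to the player for coins.
; Tick reads the cached BP_PlayerCharacter's unlock flags: once the machine gun is owned it offers the rocket launcher, then shows "Sold out" when both are owned.
; Use only returns the negative coin delta and a bought-weapon flag, leaving payment and unlocking outside this Blueprint.
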(event `self.ReceiveBeginPlay`
  (bind _asbp_player_character (cast `/Game/ThirdPersonBP/Blueprints/BP_PlayerCharacter` (`GameplayStatics.GetPlayerCharacter` 0)))
  (set `self.PlayerCharacter` _asbp_player_character))

(event `self.ReceiveTick`
  (params (DeltaSeconds :type "Float (single-precision)"))
  (bind _playercharacter (`self.PlayerCharacter`))
  (bind _text (`self.Text`))
  (if (`/Game/ThirdPersonBP/Blueprints/BP_PlayerCharacter.MachineGunUnlocked` _playercharacter)
    (if (`/Game/ThirdPersonBP/Blueprints/BP_PlayerCharacter.RocketLauncherUnlocked` _playercharacter)
      (set `self.CoinsAmount` 0)
      (`TextRenderComponent.K2_SetText` _text (`|FormatText` "Sold out"))
      (else
        (set `self.CoinsAmount` -300)
        (`TextRenderComponent.K2_SetText` _text (`KismetTextLibrary.Conv_StringToText` (`KismetStringLibrary.Concat_StrStr` (`KismetStringLibrary.Concat_StrStr` "Buy rocket launcher \n" (`KismetStringLibrary.Conv_IntToString` (* (`self.CoinsAmount`) -1))) " coins")))))))

(fn `Use`
  (returns (CoinsAmount :type Integer) (`BoughtAmmo?` :type Boolean) (`BoughtWeapon?` :type Boolean) (`BoughtGrenades?` :type Boolean) (`FoundFlamethrower?` :type Boolean))
  (return (`self.CoinsAmount`) false true false false))

(fn `UserConstructionScript`)