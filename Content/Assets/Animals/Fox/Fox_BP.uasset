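; Fox character that wanders the navmesh and flees when the player comes near.
; Tick checks player distance, raising speed and acceleration to flee when close, otherwise slowing to wander with short random pauses between moves.
; Fleeing targets a random navigable point directly away from the player, widening the search radius on failure, with flags preventing repeat requests of each move type.
; GetShot simply destroys the fox.
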(event `self.ReceiveBeginPlay`
  (bind _asplayer_character (cast `/Game/ThirdPersonBP/Blueprints/PlayerCharacter` (`GameplayStatics.GetPlayerCharacter` 0)))
  (set `self.PlayerRef` _asplayer_character))

(event `self.ReceiveTick`
  (params (DeltaSeconds :type "Float (single-precision)"))
  (bind _charactermovement (`self.CharacterMovement`))
  (if (< (`self.GetDistanceTo` (`self.PlayerRef`)) 2000.0)
    (set `CharacterMovementComponent.MaxWalkSpeed` 2000.0 _charactermovement)
    (set `CharacterMovementComponent.MaxAcceleration` 4000.0 _charactermovement)
    (`self.RunAway`)
    (else
      (set `CharacterMovementComponent.MaxWalkSpeed` 1000.0 _charactermovement)
      (set `CharacterMovementComponent.MaxAcceleration` 1000.0 _charactermovement)
      (if (not (`self.IsRunningAway`))
        (`self.MoveAround`)))))

(event `RunAway`
  (bind _returnvalue (`self.K2_GetActorLocation`))
  (bind _returnvalue_2 (`KismetMathLibrary.MakeVector` (.x (+ _returnvalue (* (`KismetMathLibrary.GetForwardVector` (`KismetMathLibrary.FindLookAtRotation` _returnvalue (`self.K2_GetActorLocation` (`self.PlayerRef`)))) -2000.0))) (.y (+ _returnvalue (* (`KismetMathLibrary.GetForwardVector` (`KismetMathLibrary.FindLookAtRotation` _returnvalue (`self.K2_GetActorLocation` (`self.PlayerRef`)))) -2000.0))) (.z _returnvalue)))
  (if (not (`self.IsRunningAway`))
    (set `self.IsRunningAway` true)
    (bind (_randomlocation _returnvalue_3) (`NavigationSystemV1.K2_GetRandomLocationInNavigableRadius` _returnvalue_2 500.0 null null))
    (if _returnvalue_3
      (`|AIMoveTo` self _randomlocation null
        (:`OnSuccess`
          _)
        (:`OnFail`
          _))
      (else
        (bind _randomlocation_2 (`NavigationSystemV1.K2_GetRandomLocationInNavigableRadius` _returnvalue_2 4000.0 null null))
        (`|AIMoveTo` self _randomlocation_2 null
          (:`OnSuccess`
            _)
          (:`OnFail`
            _))))
    (set `self.IsRunningAway` false)))

(event `MoveAround`
  (if (not (`self.IsMovingAround`))
    (set `self.IsMovingAround` true)
    (bind _randomlocation (`NavigationSystemV1.K2_GetRandomLocationInNavigableRadius` (`self.K2_GetActorLocation`) 500.0 null null))
    (`|AIMoveTo` self _randomlocation null
      (:`OnSuccess`
        _)
      (:`OnFail`
        _))
    (`KismetSystemLibrary.Delay` (`KismetMathLibrary.RandomFloatInRange` 1.0 2.0))
    (set `self.IsMovingAround` false)))

(fn `GetShot`
  (`self.K2_DestroyActor`))

(fn `UserConstructionScript`)