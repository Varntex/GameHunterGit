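; Fox animal that wanders near an assigned origin actor, flees the player, deals damage on overlapping them and drops meat when shot.
; Tick switches run, walk and idle animations through cross-resetting DoOnce gates, and sets speed by player distance, ignoring a ragdolled player.
; RunAway and MoveAround send AIMoveTo to random navigable points, away from the player (with wider fallback radius) or back toward the origin when strayed.
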(event `self.ReceiveBeginPlay`
  (bind _asbp_player_character (cast `/Game/ThirdPersonBP/Blueprints/BP_PlayerCharacter` (`GameplayStatics.GetPlayerCharacter` 0)))
  (set `self.PlayerCharacter` _asbp_player_character))

(event `self.ReceiveTick`
  (params (DeltaSeconds :type "Float (single-precision)"))
  (bind _mesh (`self.Mesh`))
  (bind _charactermovement (`self.CharacterMovement`))
  (`|ExecutionSequence`
    (:`then_0`
      (if (`self.IsRunningAway`)
        (`/Engine/EditorBlueprintResources/StandardMacros.DoOnce` false :!label _label
          (:`Completed`
            (`SkeletalMeshComponent.PlayAnimation` _mesh "/Game/Assets/Animals/Fox/MO_fox_01_Anim_Armature_run.MO_fox_01_Anim_Armature_run" true)
            (`|ExecutionSequence`
              (:`then_0`
                (goto _label_2 :!via `Reset`))
              (:`then_1`
                (goto _label_3 :!via `Reset`)))))
        (elif (`self.IsMovingAround`)
          (`/Engine/EditorBlueprintResources/StandardMacros.DoOnce` false :!label _label_2
            (:`Completed`
              (`SkeletalMeshComponent.PlayAnimation` _mesh "/Game/Assets/Animals/Fox/MO_fox_01_Anim_Armature_walk.MO_fox_01_Anim_Armature_walk" true)
              (`|ExecutionSequence`
                (:`then_0`
                  (goto _label :!via `Reset`))
                (:`then_1`
                  (goto _label_3 :!via `Reset`)))))
          (else
            (`/Engine/EditorBlueprintResources/StandardMacros.DoOnce` false :!label _label_3
              (:`Completed`
                (`SkeletalMeshComponent.PlayAnimation` _mesh "/Game/Assets/Animals/Fox/MO_fox_01_Anim_Armature_Idle.MO_fox_01_Anim_Armature_Idle" true)
                (`|ExecutionSequence`
                  (:`then_0`
                    (goto _label :!via `Reset`))
                  (:`then_1`
                    (goto _label_2 :!via `Reset`)))))))))
    (:`then_1`
      (if (`SceneComponent.IsSimulatingPhysics` (`Character.Mesh` (`self.PlayerCharacter`)) "None")
        (set `CharacterMovementComponent.MaxWalkSpeed` 1000.0 _charactermovement :!label _label_4)
        (set `CharacterMovementComponent.MaxAcceleration` 1000.0 _charactermovement)
        (if (not (`self.IsRunningAway`))
          (`KismetSystemLibrary.Delay` (`KismetMathLibrary.RandomFloatInRange` 1.0 2.0))
          (`self.MoveAround`))
        (elif (< (`self.GetDistanceTo` (`self.PlayerCharacter`)) (`self.DetectionDistance`))
          (set `CharacterMovementComponent.MaxWalkSpeed` 2000.0 _charactermovement)
          (set `CharacterMovementComponent.MaxAcceleration` 4000.0 _charactermovement)
          (`self.RunAway`)
          (else
            (goto _label_4)))))))

(event `RunAway`
  (bind _returnvalue (`self.K2_GetActorLocation`))
  (bind _returnvalue_2 (`KismetMathLibrary.MakeVector` (.x (+ _returnvalue (* (`KismetMathLibrary.GetForwardVector` (`KismetMathLibrary.FindLookAtRotation` _returnvalue (`self.K2_GetActorLocation` (`self.PlayerCharacter`)))) -4000.0))) (.y (+ _returnvalue (* (`KismetMathLibrary.GetForwardVector` (`KismetMathLibrary.FindLookAtRotation` _returnvalue (`self.K2_GetActorLocation` (`self.PlayerCharacter`)))) -4000.0))) (.z _returnvalue)))
  (if (not (`self.IsRunningAway`))
    (set `self.IsRunningAway` true)
    (bind (_randomlocation _returnvalue_3) (`NavigationSystemV1.K2_GetRandomLocationInNavigableRadius` _returnvalue_2 500.0 null null))
    (if _returnvalue_3
      (`|AIMoveTo` self _randomlocation null
        (:`OnSuccess`
          _)
        (:`OnFail`
          _))
      (else
        (bind _randomlocation_2 (`NavigationSystemV1.K2_GetRandomLocationInNavigableRadius` _returnvalue_2 8000.0 null null))
        (`|AIMoveTo` self _randomlocation_2 null
          (:`OnSuccess`
            _)
          (:`OnFail`
            _))))
    (set `self.IsRunningAway` false)))

(event `MoveAround`
  (bind _returnvalue (`self.K2_GetActorLocation`))
  (bind _returnvalue_2 (`self.GetDistanceTo` (`self.FoxOrigin`)))
  (if (not (`self.IsMovingAround`))
    (set `self.IsStandingIdle` false)
    (set `self.IsMovingAround` true)
    (if (< _returnvalue_2 (`self.OriginDistanceThreshold`))
      (bind _randomlocation (`NavigationSystemV1.K2_GetRandomLocationInNavigableRadius` (`self.K2_GetActorLocation`) 500.0 null null))
      (`|AIMoveTo` self _randomlocation null
        (:`OnSuccess`
          _)
        (:`OnFail`
          _))
      (else
        (bind _randomlocation_2 (`NavigationSystemV1.K2_GetRandomLocationInNavigableRadius` (`KismetMathLibrary.MakeVector` (.x (+ _returnvalue (* (`KismetMathLibrary.GetForwardVector` (`KismetMathLibrary.FindLookAtRotation` _returnvalue (`self.K2_GetActorLocation` (`self.FoxOrigin`)))) _returnvalue_2))) (.y (+ _returnvalue (* (`KismetMathLibrary.GetForwardVector` (`KismetMathLibrary.FindLookAtRotation` _returnvalue (`self.K2_GetActorLocation` (`self.FoxOrigin`)))) _returnvalue_2))) (.z _returnvalue)) (`self.OriginDistanceThreshold`) null null))
        (`|AIMoveTo` self _randomlocation_2 null
          (:`OnSuccess`
            _)
          (:`OnFail`
            _))))
    (set `self.IsMovingAround` false)))

(event `self.ReceiveActorBeginOverlap`
  (params (OtherActor :type "Actor Object Reference"))
  (bind _asbp_player_character (cast `/Game/ThirdPersonBP/Blueprints/BP_PlayerCharacter` OtherActor))
  (message `/Game/ThirdPersonBP/Blueprints/Interface_TakeDamage.TakeDamage` _asbp_player_character 2))

(fn `GetShot`
  (`|SpawnActorFromClass` "/Game/Assets/Animals/Fox/BP_FoxMeat.BP_FoxMeat_C" (`self.GetTransform`) "Undefined" "OverrideRootScale" null null)
  (`self.K2_DestroyActor`))

(fn `SetOrigin`
  (params (OriginActor :type "Actor Object Reference"))
  (returns (`OriginSet?` :type Boolean))
  (set `self.FoxOrigin` OriginActor)
  (return true))

(fn `UserConstructionScript`)