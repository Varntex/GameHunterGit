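; Fox spawn point that keeps a single AI fox alive around its location.
; On BeginPlay it spawns BP_Fox at a random navigable point around a center pushed away from the player by the spawn radius, then passes itself to the fox as origin.
; Tick respawns the fox through a resettable DoOnce when it is no longer valid and the player is outside the spawn radius.
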(event `self.ReceiveBeginPlay`
  (bind _asplayer_character (cast `/Game/ThirdPersonBP/Blueprints/BP_PlayerCharacter` (`GameplayStatics.GetPlayerCharacter` 0)))
  (set `self.PlayerCharacter` _asplayer_character)
  (`self.Spawn Fox`))

(event `Spawn Fox`
  (bind _returnvalue (`self.K2_GetActorLocation`))
  (bind _randomlocation (`NavigationSystemV1.K2_GetRandomLocationInNavigableRadius` (`KismetMathLibrary.MakeVector` (.x (+ _returnvalue (* (`KismetMathLibrary.GetForwardVector` (`KismetMathLibrary.FindLookAtRotation` _returnvalue (`self.K2_GetActorLocation` (`self.PlayerCharacter`)))) (* (`self.SpawnRadius`) -1.0)))) (.y (+ _returnvalue (* (`KismetMathLibrary.GetForwardVector` (`KismetMathLibrary.FindLookAtRotation` _returnvalue (`self.K2_GetActorLocation` (`self.PlayerCharacter`)))) (* (`self.SpawnRadius`) -1.0)))) (.z _returnvalue)) (`self.SpawnRadius`) null null))
  (bind _returnvalue_2 (`AIBlueprintHelperLibrary.SpawnAIFromClass` "/Game/Assets/Animals/Fox/BP_Fox.BP_Fox_C" null _randomlocation (struct) false null))
  (bind _output_get (set `self.SpawnedFox` _returnvalue_2))
  (message `/Game/Assets/Animals/SetOrigin_Interface.SetOrigin` _output_get self)
  (goto _label :!via `Reset`))

(event `self.ReceiveTick`
  (params (DeltaSeconds :type "Float (single-precision)"))
  (if (`KismetSystemLibrary.IsValid` (`self.SpawnedFox`))
    _
    (elif (not (< (`self.GetDistanceTo` (`self.PlayerCharacter`)) (`self.SpawnRadius`)))
      (`/Engine/EditorBlueprintResources/StandardMacros.DoOnce` false :!label _label
        (:`Completed`
          (`self.Spawn Fox`))))))

(fn `UserConstructionScript`)