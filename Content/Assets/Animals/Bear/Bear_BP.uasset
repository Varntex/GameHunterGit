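; Bear enemy character that wanders near an assigned origin actor until pawn sensing spots the player, then charges at them.
; Tick switches between walking and running, pausing the hunt while the player ragdolls; each charge overshoots the player's position by a fixed distance after a random delay.
; Overlapping the player deals damage and an impulse from the bear's velocity.
; Getting shot sends an unaware bear fleeing randomly, or spawns meat at zero health.
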(event `self.ReceiveBeginPlay`
  (bind _asplayer_character (cast `/Game/ThirdPersonBP/Blueprints/PlayerCharacter` (`GameplayStatics.GetPlayerCharacter` 0)))
  (set `self.PlayerCharacter` _asplayer_character))

(event `self.PawnSensing.OnSeePawn`
  (params (Pawn :type "Pawn Object Reference"))
  (if (not (`self.HasSeenPlayer`))
    (`NavMovementComponent.StopActiveMovement` (`self.CharacterMovement`))
    (set `self.HasSeenPlayer` true)))

(event `self.ReceiveTick`
  (params (DeltaSeconds :type "Float (single-precision)"))
  (bind _charactermovement (`self.CharacterMovement`))
  (if (`SceneComponent.IsSimulatingPhysics` (`Character.Mesh` (`self.PlayerCharacter`)) "None")
    (set `CharacterMovementComponent.MaxWalkSpeed` (`self.WalkSpeed`) _charactermovement :!label _label)
    (set `CharacterMovementComponent.MaxAcceleration` (`self.WalkAcceleration`) _charactermovement)
    (`self.MoveAround`)
    (elif (`self.IsAttacking`)
      _
      (elif (`self.IsRunningRandom`)
        _
        (elif (`self.HasSeenPlayer`)
          (set `CharacterMovementComponent.MaxWalkSpeed` (`self.RunSpeed`) _charactermovement)
          (set `CharacterMovementComponent.MaxAcceleration` (`self.RunAcceleration`) _charactermovement)
          (`self.Attack`)
          (else
            (goto _label)))))))

(event `Attack`
  (bind _returnvalue (`self.K2_GetActorLocation`))
  (bind _playercharacter (`self.PlayerCharacter`))
  (if (not (`self.IsAttacking`))
    (set `self.IsAttacking` true)
    (`self.K2_SetActorRotation` (`KismetMathLibrary.MakeRotator` (.roll (`KismetMathLibrary.FindLookAtRotation` (`self.K2_GetActorLocation`) (`self.K2_GetActorLocation` (`self.PlayerCharacter`)))) 0.0 (.yaw (`KismetMathLibrary.FindLookAtRotation` (`self.K2_GetActorLocation`) (`self.K2_GetActorLocation` (`self.PlayerCharacter`))))))
    (`KismetSystemLibrary.Delay` (`KismetMathLibrary.RandomFloatInRange` 0.0 1.0))
    (`|AIMoveTo` self (+ _returnvalue (* (`KismetMathLibrary.GetForwardVector` (`KismetMathLibrary.FindLookAtRotation` _returnvalue (`self.K2_GetActorLocation` _playercharacter))) (+ (`self.GetDistanceTo` _playercharacter) 500.0))) null
      (:`OnSuccess`
        _)
      (:`OnFail`
        _))
    (set `self.IsAttacking` false)))

(event `MoveAround`
  (bind _returnvalue (`KismetMathLibrary.RandomFloatInRange` 1.0 2.0))
  (bind _returnvalue_2 (`self.K2_GetActorLocation`))
  (bind _returnvalue_3 (`self.GetDistanceTo` (`self.BearOrigin`)))
  (if (not (`self.IsMovingAround`))
    (set `self.IsMovingAround` true)
    (if (< _returnvalue_3 (`self.OriginDistanceThreshold`))
      (bind _randomlocation (`NavigationSystemV1.K2_GetRandomLocationInNavigableRadius` (`self.K2_GetActorLocation`) 500.0 null null))
      (`|AIMoveTo` self _randomlocation null
        (:`OnSuccess`
          _)
        (:`OnFail`
          _))
      (`KismetSystemLibrary.Delay` _returnvalue)
      (set `self.IsMovingAround` false)
      (else
        (bind _randomlocation_2 (`NavigationSystemV1.K2_GetRandomLocationInNavigableRadius` (`KismetMathLibrary.MakeVector` (.x (+ _returnvalue_2 (* (`KismetMathLibrary.GetForwardVector` (`KismetMathLibrary.FindLookAtRotation` _returnvalue_2 (`self.K2_GetActorLocation` (`self.BearOrigin`)))) _returnvalue_3))) (.y (+ _returnvalue_2 (* (`KismetMathLibrary.GetForwardVector` (`KismetMathLibrary.FindLookAtRotation` _returnvalue_2 (`self.K2_GetActorLocation` (`self.BearOrigin`)))) _returnvalue_3))) (.z _returnvalue_2)) (`self.OriginDistanceThreshold`) null null))
        (`|AIMoveTo` self _randomlocation_2 null
          (:`OnSuccess`
            _)
          (:`OnFail`
            _))
        (`KismetSystemLibrary.Delay` _returnvalue)
        (set `self.IsMovingAround` false)))))

(event `RunRandom`
  (bind _charactermovement (`self.CharacterMovement`))
  (set `self.IsRunningRandom` true)
  (set `CharacterMovementComponent.MaxWalkSpeed` (`self.RunSpeed`) _charactermovement)
  (set `CharacterMovementComponent.MaxAcceleration` (`self.RunAcceleration`) _charactermovement)
  (`|AIMoveTo` self (`NavigationSystemV1.K2_GetRandomLocationInNavigableRadius` (`self.K2_GetActorLocation`) 10000.0 null null) null
    (:`OnSuccess`
      _)
    (:`OnFail`
      _))
  (set `self.IsRunningRandom` false))

(event `self.ReceiveActorBeginOverlap`
  (params (OtherActor :type "Actor Object Reference"))
  (bind _asplayer_character (cast `/Game/ThirdPersonBP/Blueprints/PlayerCharacter` OtherActor))
  (message `/Game/ThirdPersonBP/Blueprints/TakeDamage_Interface.TakeDamage` _asplayer_character 9)
  (`CharacterMovementComponent.AddImpulse` (`Character.CharacterMovement` _asplayer_character) (`self.GetVelocity`) false))

(fn `GetShot`
  (bind _output_get (set `self.Health` (- (`self.Health`) 1)))
  (if (<= _output_get 0)
    (`|SpawnActorFromClass` "/Game/Assets/Animals/Bear/BearMeat_BP.BearMeat_BP_C" (`self.GetTransform`) "Undefined" "OverrideRootScale" null null)
    (`self.K2_DestroyActor`)
    (elif (not (`self.HasSeenPlayer`))
      (`self.RunRandom`))))

(fn `SetOrigin`
  (params (OriginActor :type "Actor Object Reference"))
  (returns (`OriginSet?` :type Boolean))
  (set `self.BearOrigin` OriginActor)
  (return true))

(fn `TakeDamage`
  (returns (`TookDamage?` :type Boolean))
  (return false))

(fn `UserConstructionScript`)